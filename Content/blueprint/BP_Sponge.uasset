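; BP_Sponge is a sponge for cleaning blood that has a limited number of uses before it must be wrung out.
; It refills UsesLeft from MaxUses on BeginPlay.
; Each CleanedBlood event decrements the counter and clears CanClean once it runs out.
; WringSponge restores the uses and sets CanClean again.
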(event `self.ReceiveBeginPlay`
  (set `self.usesLeft` (`self.maxUses`)))

(event `CleanedBlood`
  (bind _result (`/Engine/EditorBlueprintResources/StandardMacros.DecrementInt` (`self.usesLeft`))
    (:`  `
      (if (<= _result 0)
        (set `self.canClean` false)))))

(event `WringSponge`
  (set `self.canClean` true)
  (set `self.usesLeft` (`self.maxUses`)))

(fn `UserConstructionScript`)