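; BP_testBloodStains is a test actor that leaves blood splatter decals where particles hit surfaces.
; On BeginPlay it attaches the Splatter_PS emitter slightly above its root and binds to its particle collision event.
; Each collision spawns a decal aligned to the hit normal, with random size and a dynamic material instance whose Frame parameter picks a random splatter variant.
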(event `self.ReceiveBeginPlay`
  (bind _returnvalue (`GameplayStatics.SpawnEmitterAttached` "/Game/BloodStains/splatter_PS.splatter_PS" (`self.DefaultSceneRoot`) "None" (0.0 0.0 50.0)))
  (add `ParticleSystemComponent.OnParticleCollide` _returnvalue (delegate `On Collide Event`)))

(event `On Collide Event`
  (params (EventName :type Name) (EmitterTime :type "Float (double-precision)") (ParticleTime :type Integer) (Location :type "Vector Structure") (Velocity :type "Vector Structure") (Direction :type "Vector Structure") (Normal :type "Vector Structure") (BoneName :type Name) (PhysMat :type "PhysicalMaterial Object Reference"))
  (bind _returnvalue (`KismetMaterialLibrary.CreateDynamicMaterialInstance` "/Game/BloodStains/splatters_decal_M.splatters_decal_M"))
  (`MaterialInstanceDynamic.SetScalarParameterValue` _returnvalue "Frame" (`KismetMathLibrary.Conv_IntToDouble` (`KismetMathLibrary.RandomInteger` 11)))
  (`GameplayStatics.SpawnDecalAtLocation` _returnvalue (`KismetMathLibrary.Conv_DoubleToVector` (`KismetMathLibrary.RandomFloatInRange` 20.0 50.0)) Location (`KismetMathLibrary.Conv_VectorToRotator` Normal)))

(fn `UserConstructionScript`)